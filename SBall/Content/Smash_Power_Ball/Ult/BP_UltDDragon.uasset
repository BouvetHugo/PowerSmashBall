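; Dragon ultimate actor that emerges from a portal and flies toward the player's camera ray target.
; UltiCalled spawns a BP_Portal facing that target and scales it up by timeline, then launches the dragon through ProjectileMovement and calls EndOfUlt on the character.
; Timelines drive Material Parameter Collection scalars for the dragon's appearance radius and distortion.
; Delayed timelines later shrink the portal and destroy both actors.
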(event `UltiCalled`
  ;[1 1 1] Dragon goes on the ray cast camera and trotate to look at it
  (`KismetMaterialLibrary.SetScalarParameterValue` "/Game/Smash_Power_Ball/Ult/Materials_Shaders/Coll_DragonScalar.Coll_DragonScalar" "Radius" 90.0)
  (bind _asthird_person_character (cast `/Game/ThirdPersonBP/Blueprints/ThirdPersonCharacter` (`GameplayStatics.GetPlayerCharacter` 0)))
  (set `self.Character` _asthird_person_character)
  (set `self.LookRotation` (`KismetMathLibrary.RInterpTo` (`self.K2_GetActorRotation`) (`KismetMathLibrary.FindLookAtRotation` (`self.K2_GetActorLocation`) (`/Game/ThirdPersonBP/Blueprints/ThirdPersonCharacter.CamRay` _asthird_person_character)) (`GameplayStatics.GetWorldDeltaSeconds`)))
  (bind _returnvalue (`|SpawnActorFromClass` "/Game/Smash_Power_Ball/Ult/Materials_Shaders/BP_Portal.BP_Portal_C" (`KismetMathLibrary.MakeTransform` (`self.K2_GetActorLocation`) (`self.LookRotation`) (0.0 0.0 0.0)) "Undefined" "OverrideRootScale" null null))
  (bind _output_get (set `self.Portal` _returnvalue))
  (bind (_direction _newtrack_0) (`Timeline|TimeScale` :!via `PlayFromStart`)
    (:`Update`
      (`self.SetActorScale3D` _output_get (`KismetMathLibrary.VLerp` (0.0 0.0 0.0) (2.5 2.5 2.5) _newtrack_0)))
    (:`Finished`
      (`|ExecutionSequence`
        (:`then_0`
          (bind _asthird_person_character_2 (cast `/Game/ThirdPersonBP/Blueprints/ThirdPersonCharacter` (`GameplayStatics.GetPlayerCharacter` 0)))
          (set `MovementComponent.Velocity` (* (`KismetMathLibrary.Normal` (- (`/Game/ThirdPersonBP/Blueprints/ThirdPersonCharacter.CamRay` _asthird_person_character_2) (`self.K2_GetActorLocation`))) (`self.Speed`)) (`self.ProjectileMovement`)))
        (:`then_1`
          (bind (_direction_2 _newtrack_0_2) (`Timeline|DragonAppears` :!via `PlayFromStart`)
            (:`Update`
              (`KismetMaterialLibrary.SetScalarParameterValue` "/Game/Smash_Power_Ball/Ult/Materials_Shaders/Coll_DragonScalar.Coll_DragonScalar" "Radius" _newtrack_0_2))))
        (:`then_2`
          (`self.K2_SetActorRotation` (`self.LookRotation`)))
        (:`then_3`
          (bind (_direction_3 _distorsion) (`Timeline|DragonDistorsion` :!via `PlayFromStart`)
            (:`Update`
              (`KismetMaterialLibrary.SetScalarParameterValue` "/Game/Smash_Power_Ball/Ult/Materials_Shaders/Coll_DragonDistorsion.Coll_DragonDistorsion" "Scalar" _distorsion))))
        (:`then_4`
          (`KismetSystemLibrary.Delay` 9.0)
          (`Timeline|TimeDestroy` :!via `PlayFromStart`
            (:`Finished`
              (`self.K2_DestroyActor` (`self.Portal`))
              (`self.K2_DestroyActor`))))
        (:`then_5`
          (`/Game/ThirdPersonBP/Blueprints/ThirdPersonCharacter.EndOfUlt` (`self.Character`)))
        (:`then_6`
          (`KismetSystemLibrary.Delay` 5.0)
          (bind (_direction_4 _newtrack_0_3) (`Timeline|Timeline_0` :!via `PlayFromStart`)
            (:`Update`
              (`self.SetActorScale3D` (`self.Portal`) (`KismetMathLibrary.VLerp` (3.0 3.0 3.0) (0.0 0.0 0.0) _newtrack_0_3)))))))))

(fn `UserConstructionScript`)